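; BP_Player is a mouse-aimed, physics-driven player that destroys any BP_Timsah actor it begins overlapping.
; It shows the cursor on BeginPlay, then each tick projects the Karakter component to screen space and computes the angle to the mouse with Atan2.
; That angle becomes the roll of the PhysicsConstraint's angular orientation target, so rotation is driven through the constraint instead of set directly.
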(event `self.ReceiveBeginPlay`
  (set `PlayerController.bShowMouseCursor` true (`GameplayStatics.GetPlayerController` 0)))

(event `self.ReceiveTick`
  (params (DeltaSeconds :type "Float (single-precision)"))
  (bind (_locationx _locationy) (`PlayerController.GetMousePosition` (`GameplayStatics.GetPlayerController` 0)))
  (bind _screenposition (`GameplayStatics.ProjectWorldToScreen` (`GameplayStatics.GetPlayerController` 0) (`SceneComponent.K2_GetComponentLocation` (`self.karakter`)) true))
  (`PhysicsConstraintComponent.SetAngularOrientationTarget` (`self.PhysicsConstraint`) (`KismetMathLibrary.MakeRotator` (`KismetMathLibrary.DegAtan2` (- _locationy (`.Y` (`KismetMathLibrary.BreakVector2D` _screenposition))) (- _locationx (`KismetMathLibrary.BreakVector2D` _screenposition))))))

(event `self.ReceiveActorBeginOverlap`
  (params (OtherActor :type "Actor Object Reference"))
  (bind _asbp_timsah (cast `/Game/Timsah/BP_Timsah` OtherActor))
  (`self.K2_DestroyActor` _asbp_timsah))

(fn `UserConstructionScript`)